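; BP_Zombie is a wave-mode enemy that chases the player and deals melee damage.
; An AIMoveTo loop targeting the player controller leads into an attack montage, whose notify triggers a sound and sphere-overlap damage check before the chase resumes.
; Point damage plays a hit reaction or, at zero health, awards points, loosens collision, plays death, notifies WaveMode and destroys the actor after a delay.
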(event `self.ReceiveBeginPlay`
  (`self.RunToPlayer`))

(event `RunToPlayer`
  ;[1 1 1] Run to player
  (if (not (`self.isDead`))
    (`|AIMoveTo` self (0.0 0.0 0.0) (`GameplayStatics.GetPlayerController` 0) 40.0
      (:`OnSuccess`
        (`self.AttackPlayer`))
      (:`OnFail`
        (`self.RunToPlayer`)))))

(event `AttackPlayer`
  ;[1 1 1] Attack player
  (`|PlayMontage` (`self.Mesh`) "/Game/_Main/Zombie/Animations/zombie_attack_Montage1.zombie_attack_Montage1"
    (:`OnCompleted`
      (`self.RunToPlayer` :!label _label))
    (:`OnInterrupted`
      (goto _label))
    (:`OnNotifyBegin`
      (`GameplayStatics.PlaySoundAtLocation` "/Game/_Main/Zombie/Sounds/AttackCue.AttackCue" (`self.K2_GetActorLocation`) (struct) 1.0 1.0 0.0 "/Game/MilitaryWeapSilver/Sound/Attenuation/WeaponShot_att.WeaponShot_att" null null null)
      (bind (_outactors _returnvalue) (`KismetSystemLibrary.SphereOverlapActors` (`SceneComponent.K2_GetComponentLocation` (`self.Arrow1`)) 80.0 (`|MakeArray` "ObjectTypeQuery3" :!type "EObjectTypeQuery Enum") "/Game/_Main/Blueprints/BP_FirstPersonCharacter.BP_FirstPersonCharacter_C" (`|MakeArray` self :!type "Actor Object Reference")))
      (if _returnvalue
        (for _array_element _outactors
          (`GameplayStatics.ApplyDamage` _array_element 50.0 (`self.GetController`) self "/Script/Engine.DamageType"))))))

(event `self.ReceivePointDamage`
  (params (Damage :type "Float (single-precision)") (DamageType :type "DamageType Object Reference") (HitLocation :type "Vector Structure") (HitNormal :type "Vector Structure") (HitComponent :type "PrimitiveComponent Object Reference") (BoneName :type Name) (ShotFromDirection :type "Vector Structure") (InstigatedBy :type "Controller Object Reference") (DamageCauser :type "Actor Object Reference") (HitInfo :type "HitResult Structure (by ref)"))
  (bind _health (`self.health`))
  ;[1 1 1] Take damage
  (if (not (`self.isDead`))
    (set `self.health` (`KismetMathLibrary.FTrunc` (- _health Damage)))
    (if (<= _health 0)
      (`self.Death`)
      (bind _asbp_first_person_character (cast `/Game/_Main/Blueprints/BP_FirstPersonCharacter` (`GameplayStatics.GetPlayerCharacter` 0)))
      (set `/Game/_Main/Blueprints/BP_FirstPersonCharacter.points` (+ (`/Game/_Main/Blueprints/BP_FirstPersonCharacter.points` _asbp_first_person_character) 50) _asbp_first_person_character)
      (else
        (`|PlayMontage` (`self.Mesh`) "/Game/_Main/Zombie/Animations/Zombie_Reaction_Hit_mixamo_com_Montage.Zombie_Reaction_Hit_mixamo_com_Montage")))))

(event `Death`
  (bind _capsulecomponent (`self.CapsuleComponent`))
  ;[1 1 1] Death
  (set `self.isDead` true)
  (`MovementComponent.StopMovementImmediately` (`self.CharacterMovement`))
  (`PrimitiveComponent.SetCollisionResponseToChannel` _capsulecomponent "ECC_Camera" "ECR_Ignore")
  (`PrimitiveComponent.SetCollisionResponseToChannel` _capsulecomponent "ECC_Pawn" "ECR_Overlap")
  (`PrimitiveComponent.SetCollisionEnabled` (`self.Mesh`) "NoCollision")
  (`|PlayMontage` (`self.Mesh`) "/Game/_Main/Zombie/Animations/zombie_dying_Montage.zombie_dying_Montage"
    (:`then`
      (bind _aswave_mode (cast `/Game/_Main/Blueprints/WaveMode` (`GameplayStatics.GetGameMode`)))
      (`/Game/_Main/Blueprints/WaveMode.ZombieKilled` _aswave_mode)
      (`KismetSystemLibrary.Delay` 5.0)
      (`self.K2_DestroyActor`))))

(fn `UserConstructionScript`)