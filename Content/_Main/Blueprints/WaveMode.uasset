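; Wave-based zombie survival logic that starts on BeginPlay, setting game-only input and player walk speed, then launching the first wave.
; Each wave spawns zombies through a delayed-loop macro at two fixed points, scaling count and health with wave number and speed in tiers.
; ZombieKilled counts down the remainder and starts the next wave after a sound and pause.
; BlockZombies switches tracked zombies to a looping idle animation.
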(event `self.ReceiveBeginPlay`
  ;[1 1 1] Start game
  (`self.StartGame`))

(event `StartGame`
  (bind _returnvalue (`GameplayStatics.GetPlayerController` 0))
  ;[1 1 1] Start game
  (set `PlayerController.bShowMouseCursor` false _returnvalue)
  (`WidgetBlueprintLibrary.SetInputMode_GameOnly` _returnvalue)
  (set `CharacterMovementComponent.MaxWalkSpeed` 300.0 (`Character.CharacterMovement` (`GameplayStatics.GetPlayerCharacter` 0)))
  (`self.WaveIncrement`))

(event `SpawnZombies`
  (bind _currentwave (`self.currentWave`))
  (bind _currentwave_2 (`self.currentWave`))
  ;[1 1 1] Spawn zombies
  (bind _output_get (set `self.zombiesNumber` (* _currentwave 5)))
  (set `self.zombiesLeft` _output_get)
  (set `self.zombieHealth` (+ (* (- _currentwave 1) 12) 100))
  (`self.ForLoopWithDelay` 1 _output_get 1.57
    (:`loop body`
      (if (== (`KismetMathLibrary.RandomInteger` 3) 0)
        (set `self.spawnLocation` (`KismetMathLibrary.MakeTransform` (`KismetMathLibrary.MakeVector` 9200.0 18300.0 188.0)))
        (else
          (set `self.spawnLocation` (`KismetMathLibrary.MakeTransform` (`KismetMathLibrary.MakeVector` 5300.0 18500.0 188.0)))))
      (bind _returnvalue (`|SpawnActorFromClass` "/Game/_Main/Zombie/BP_Zombie.BP_Zombie_C" (`self.spawnLocation`) "AlwaysSpawn" "OverrideRootScale" null null))
      (`KismetArrayLibrary.Array_Add` (`self.zombies`) _returnvalue)
      (set `/Game/_Main/Zombie/BP_Zombie.health` (`self.zombieHealth`) _returnvalue)
      (if (< _currentwave_2 5)
        (bind _charactermovement (`Character.CharacterMovement` _returnvalue))
        (set `CharacterMovementComponent.MaxWalkSpeed` 100.0 _charactermovement)
        (elif (and (>= _currentwave_2 5) (< _currentwave_2 10))
          (set `CharacterMovementComponent.MaxWalkSpeed` 200.0 _charactermovement)
          (else
            (set `CharacterMovementComponent.MaxWalkSpeed` 400.0 _charactermovement)))))))

(event `ZombieKilled`
  (params (zombie :type "Actor Object Reference"))
  ;[1 1 1] Zombie killed
  (`KismetArrayLibrary.Array_RemoveItem` (`self.zombies`) zombie)
  (bind _result (`/Engine/EditorBlueprintResources/StandardMacros.DecrementInt` (`self.zombiesLeft`))
    (:`  `
      (if (== _result 0)
        (`GameplayStatics.PlaySound2D` "/Game/_Main/Sounds/end_round.end_round" 1.0 1.0 0.0 null null)
        (`KismetSystemLibrary.Delay` 8.0)
        (`self.WaveIncrement`)))))

(event `WaveIncrement`
  ;[1 1 1] Wave change
  (`/Engine/EditorBlueprintResources/StandardMacros.IncrementInt` (`self.currentWave`)
    (:`  `
      (`KismetSystemLibrary.Delay` 1.0)
      (`GameplayStatics.PlaySound2D` "/Game/_Main/Sounds/starting_round.starting_round" 0.5 1.0 0.0 null null)
      (`KismetSystemLibrary.Delay` 10.0)
      (`self.SpawnZombies`))))

(event `BlockZombies`
  ;[1 1 1] Block zombies movements
  (for _array_element (`self.zombies`)
    (bind _asbp_zombie (cast `/Game/_Main/Zombie/BP_Zombie` _array_element))
    (`SkeletalMeshComponent.PlayAnimation` (`Character.Mesh` _asbp_zombie) "/Game/_Main/Zombie/Furry/Gren/Animations/furry_zombie_idle.furry_zombie_idle" true)))

(fn `UserConstructionScript`)