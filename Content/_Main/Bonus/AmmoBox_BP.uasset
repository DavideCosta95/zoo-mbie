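; AmmoBox_BP is a purchase point where the first-person character buys an ammo refill with points.
; Its Box overlap events show and hide the buy-ammo interact message on the character.
; Interact refills overlapping characters whose total ammo differs from the fixed maximum, deducting a fixed point cost without checking their balance.
; It also triggers a reload if the current ammo is empty.
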(event `/Game/_Main/Blueprints/InteractInterface.Interact`
  ;[1 1 1] Interact
  (for _array_element (`PrimitiveComponent.GetOverlappingActors` (`self.Box`) "/Game/_Main/Blueprints/BP_FirstPersonCharacter.BP_FirstPersonCharacter_C")
    (bind _asbp_first_person_character (cast `/Game/_Main/Blueprints/BP_FirstPersonCharacter` _array_element))
    (if (not (== (`/Game/_Main/Blueprints/BP_FirstPersonCharacter.totalAmmo` _asbp_first_person_character) 80))
      (set `/Game/_Main/Blueprints/BP_FirstPersonCharacter.points` (- (`/Game/_Main/Blueprints/BP_FirstPersonCharacter.points` _asbp_first_person_character) 1000) _asbp_first_person_character)
      (set `/Game/_Main/Blueprints/BP_FirstPersonCharacter.totalAmmo` 80 _asbp_first_person_character)
      (if (== (`/Game/_Main/Blueprints/BP_FirstPersonCharacter.currentAmmo` _asbp_first_person_character) 0)
        (`/Game/_Main/Blueprints/BP_FirstPersonCharacter.Reload` _asbp_first_person_character)))))

(event `self.Box.OnComponentBeginOverlap`
  (params (OverlappedComponent :type "PrimitiveComponent Object Reference") (OtherActor :type "Actor Object Reference") (OtherComp :type "PrimitiveComponent Object Reference") (OtherBodyIndex :type Integer) (bFromSweep :type Boolean) (SweepResult :type "HitResult Structure (by ref)"))
  ;[1 1 1] Overlap handlers
  (bind _asbp_first_person_character (cast `/Game/_Main/Blueprints/BP_FirstPersonCharacter` OtherActor))
  (`/Game/_Main/Blueprints/BP_FirstPersonCharacter.ShowBuyAmmoInteractMessage` _asbp_first_person_character))

(event `self.Box.OnComponentEndOverlap`
  (params (OverlappedComponent :type "PrimitiveComponent Object Reference") (OtherActor :type "Actor Object Reference") (OtherComp :type "PrimitiveComponent Object Reference") (OtherBodyIndex :type Integer))
  ;[1 1 1] Overlap handlers
  (bind _asbp_first_person_character (cast `/Game/_Main/Blueprints/BP_FirstPersonCharacter` OtherActor))
  (`/Game/_Main/Blueprints/BP_FirstPersonCharacter.HideInteractMessage` _asbp_first_person_character))

(fn `UserConstructionScript`)