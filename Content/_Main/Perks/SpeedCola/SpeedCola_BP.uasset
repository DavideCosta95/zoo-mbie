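; Speed Cola perk pickup that sells faster reloading to the player, in the style of a perk machine.
; Overlapping its Box shows or hides the interact prompt.
; Interact fires once per instance, deducting Cost from the Points of overlapping first-person characters without a balance check, doubling their ReloadingSpeed and calling ActiveSpeedCola.
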(event `/Game/_Main/Blueprints/InteractInterface.Interact`
  (`/Engine/EditorBlueprintResources/StandardMacros.DoOnce` false
    (:`Completed`
      (for _array_element (`PrimitiveComponent.GetOverlappingActors` (`self.Box`) "/Game/_Main/Blueprints/BP_FirstPersonCharacter.BP_FirstPersonCharacter_C")
        (bind _asbp_first_person_character (cast `/Game/_Main/Blueprints/BP_FirstPersonCharacter` _array_element))
        (set `/Game/_Main/Blueprints/BP_FirstPersonCharacter.points` (- (`/Game/_Main/Blueprints/BP_FirstPersonCharacter.points` _asbp_first_person_character) (`self.cost`)) _asbp_first_person_character)
        (set `/Game/_Main/Blueprints/BP_FirstPersonCharacter.reloadingSpeed` (* (`/Game/_Main/Blueprints/BP_FirstPersonCharacter.reloadingSpeed` _asbp_first_person_character) 2.0) _asbp_first_person_character)
        (`/Game/_Main/Blueprints/BP_FirstPersonCharacter.ActiveSpeedCola` _asbp_first_person_character)))))

(event `self.Box.OnComponentBeginOverlap`
  (params (OverlappedComponent :type "PrimitiveComponent Object Reference") (OtherActor :type "Actor Object Reference") (OtherComp :type "PrimitiveComponent Object Reference") (OtherBodyIndex :type Integer) (bFromSweep :type Boolean) (SweepResult :type "HitResult Structure (by ref)"))
  (cast `/Game/_Main/Blueprints/BP_FirstPersonCharacter` OtherActor)
  (`SceneComponent.SetHiddenInGame` (`self.SpeedColaInteractText`) false false))

(event `self.Box.OnComponentEndOverlap`
  (params (OverlappedComponent :type "PrimitiveComponent Object Reference") (OtherActor :type "Actor Object Reference") (OtherComp :type "PrimitiveComponent Object Reference") (OtherBodyIndex :type Integer))
  (cast `/Game/_Main/Blueprints/BP_FirstPersonCharacter` OtherActor)
  (`SceneComponent.SetHiddenInGame` (`self.SpeedColaInteractText`) true false))

(fn `UserConstructionScript`)